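; Prototype invisibility power pickup that clears the IsVisible flag on the actor passed to it.
; A looping timer started at BeginPlay appears to drive RotateCoin, which spins the Cylinder mesh in small roll steps.
; ActivatePower sets the flag and destroys the Sphere and Cylinder components.
; It ends in a five-second delay with nothing after it, so visibility is never restored here.
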(event Custom|RotateCoin
  (Transformation|AddRelativeRotation (Variables|Default|GetCylinder) (Math|Rotator|MakeRotator 1e+01 0.0 0.0) false false))

(event EventBeginPlay
  (Utilities|Time|SetTimerbyEvent (EventDispatchers|CreateEvent :!event Custom|RotateCoin) 0.1 true))

(event EventActivatePower
  (params (Actor :type BP%20PC%20Object%20Reference))
  (Variables|/Game/_Test/ProtoTyping/Pawns/BP_PC.BP_PC_C|SetIsVisible Actor false)
  (Components|DestroyComponent (Variables|Default|GetSphere))
  (Utilities|FlowControl|Delay 5.0))

(fn ConstructionScript)