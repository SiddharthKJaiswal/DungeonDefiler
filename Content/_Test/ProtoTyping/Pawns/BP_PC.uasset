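; BP_PC is a prototype player character with Enhanced Input movement, look and jump that picks up collectables and power-ups.
; BeginPlay adds the default mapping context and a weapon component and caches the main game mode, while the shoot input is an empty stub.
; Capsule overlaps use interface checks to identify pickups, activate powers on the player, notify the game mode, then destroy the pickup.
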(event OnComponentBeginOverlap(CapsuleComponent)
  (params (OverlappedComponent :type Primitive%20Component%20Object%20Reference) (OtherActor :type Actor%20Object%20Reference) (OtherComp :type Primitive%20Component%20Object%20Reference) (OtherBodyIndex :type Integer) (bFromSweep :type Boolean) (SweepResult :type Hit%20Result%20Structure%20%28by%20ref%29))
  (if (Utilities|DoesObjectImplementInterface OtherActor "/Game/_Test/ProtoTyping/Items/BPI_Collectable.BPI_Collectable_C")
    (Default|CollectablesCollected (Variables|Default|GetRefrence_GameMode))
    (Actor|DestroyActor OtherActor :!label _label)
    (elif (Utilities|DoesObjectImplementInterface OtherActor "/Game/_Test/ProtoTyping/Items/BPI_Power.BPI_Power_C")
      (Class|BPIPower|ActivatePower(Message) OtherActor self)
      (Default|PowerUpUsed (Variables|Default|GetRefrence_GameMode))
      (goto _label))))

(event Input|EnhancedActionEvents|EnhancedInputActionIA_Move
  (params (ActionValue :type Vector%202D%20Structure) (ElapsedSeconds :type Float%20%28double-precision%29) (TriggeredSeconds :type Float%20%28double-precision%29) (InputAction :type Input%20Action%20Object%20Reference :default "/Game/_Test/ProtoTyping/Inputs/Actions/IA_Move.IA_Move"))
  (bind _returnvalue (Pawn|GetControlRotation :!class /Script/Engine.Pawn))
  (Pawn|Input|AddMovementInput (Math|Vector|GetRightVector (Math|Rotator|MakeRotator (.roll _returnvalue) 0.0 (.yaw _returnvalue))) (.x ActionValue) false)
  (Pawn|Input|AddMovementInput (Math|Vector|GetForwardVector (Math|Rotator|MakeRotator 0.0 0.0 (.yaw (Pawn|GetControlRotation :!class /Script/Engine.Pawn)))) (.y ActionValue) false))

(event Input|EnhancedActionEvents|EnhancedInputActionIA_Look
  (params (ActionValue :type Vector%202D%20Structure) (ElapsedSeconds :type Float%20%28double-precision%29) (TriggeredSeconds :type Float%20%28double-precision%29) (InputAction :type Input%20Action%20Object%20Reference :default "/Game/_Test/ProtoTyping/Inputs/Actions/IA_Look.IA_Look"))
  (Pawn|Input|AddControllerYawInput (.x ActionValue))
  (Pawn|Input|AddControllerPitchInput (.y ActionValue)))

(event Input|EnhancedActionEvents|EnhancedInputActionIA_Jump
  (params (ActionValue :type Boolean) (ElapsedSeconds :type Float%20%28double-precision%29) (TriggeredSeconds :type Float%20%28double-precision%29) (InputAction :type Input%20Action%20Object%20Reference :default "/Game/_Test/ProtoTyping/Inputs/Actions/IA_Jump.IA_Jump"))
  (if ActionValue
    (Character|Jump)
    (else
      (Character|StopJumping))))

(event Input|EnhancedActionEvents|EnhancedInputActionIA_Shoot
  (params (ActionValue :type Boolean) (ElapsedSeconds :type Float%20%28double-precision%29) (TriggeredSeconds :type Float%20%28double-precision%29) (InputAction :type Input%20Action%20Object%20Reference :default "/Game/_Test/FirstPerson/Input/Actions/IA_Shoot.IA_Shoot")))

(event EventBeginPlay
  (bind _asplayer_controller (Utilities|Casting|CastToPlayerController (Pawn|GetController)))
  (Input|AddMappingContext (PlayerController|LocalPlayerSubsystems|GetEnhancedInputLocalPlayerSubsystem _asplayer_controller) "/Game/_Test/ProtoTyping/Inputs/IMC_Default.IMC_Default" 0 "(bIgnoreAllPressedKeysUntilRelease=True,bForceImmediately=False,bNotifyUserSettings=False)")
  (AddComponent|AddBPWeaponComponent false)
  (bind _asbp_game_mode_main_game (Utilities|Casting|CastToBP_GameMode_MainGame (Game|GetGameMode)))
  (Variables|Default|SetRefrence_GameMode _asbp_game_mode_main_game))

(fn ConstructionScript)