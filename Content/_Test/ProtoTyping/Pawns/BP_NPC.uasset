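; Prototype enemy NPC pawn that chases the player and reports a loss to the main game mode when its Box overlaps a visible player.
; PawnSensing sight triggers AIMoveTo toward visible players; hearing only computes a look-at rotation, as the turning logic is disconnected from Tick.
; On death it ragdolls, disables sensing and collision components, notifies the game mode of the kill, then destroys itself after a delay.
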(event OnSeePawn(PawnSensing)
  (params (Pawn :type Pawn%20Object%20Reference))
  (bind _asbp_pc (Utilities|Casting|CastToBP_PC Pawn))
  (if (Variables|/Game/_Test/ProtoTyping/Pawns/BP_PC.BP_PC_C|GetIsVisible _asbp_pc)
    (AI|AIMoveTo self (Pawn|GetNavAgentLocation _asbp_pc) 0 5.0 false)))

(event OnComponentBeginOverlap(Box)
  (params (OverlappedComponent :type Primitive%20Component%20Object%20Reference) (OtherActor :type Actor%20Object%20Reference) (OtherComp :type Primitive%20Component%20Object%20Reference) (OtherBodyIndex :type Integer) (bFromSweep :type Boolean) (SweepResult :type Hit%20Result%20Structure%20%28by%20ref%29))
  (bind _asbp_pc (Utilities|Casting|CastToBP_PC OtherActor))
  (if (Variables|/Game/_Test/ProtoTyping/Pawns/BP_PC.BP_PC_C|GetIsVisible _asbp_pc)
    (bind _asbp_game_mode_main_game (Utilities|Casting|CastToBP_GameMode_MainGame (Game|GetGameMode)))
    (Default|GameEnd _asbp_game_mode_main_game false self)))

(event OnHearNoise(PawnSensing)
  (params (Instigator :type Pawn%20Object%20Reference) (Location :type Vector%20%28by%20ref%29 :default "0, 0, 0") (Volume :type Float%20%28single-precision%29))
  (Variables|Default|SetLookAt (Math|Rotator|FindLookatRotation (Transformation|GetActorLocation) Location)))

(event EventOnDeath
  (Physics|SetSimulatePhysics (Variables|Character|GetMesh) true)
  (Components|Activation|Deactivate (Variables|Default|GetPawnSensing))
  (Components|Activation|Deactivate (Variables|Collision|GetCapsuleComponent))
  (Components|DestroyComponent (Variables|Default|GetBox))
  (bind _asbp_game_mode_main_game (Utilities|Casting|CastToBP_GameMode_MainGame (Game|GetGameMode)))
  (Default|NPCKilled _asbp_game_mode_main_game)
  (Utilities|FlowControl|Delay 3.0)
  (Actor|DestroyActor))

(event EventTick
  (params (DeltaSeconds :type Float%20%28single-precision%29)))

(fn ConstructionScript)