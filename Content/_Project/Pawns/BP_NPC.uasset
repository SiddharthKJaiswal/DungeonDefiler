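; BP_NPC is an enemy pawn that chases the player on sight and ends the game as a loss when it reaches them.
; Pawn sensing drives the AI move, and the game mode receives the game end and kill notifications.
; On death it ragdolls, notifies the game mode and is destroyed after a delay.
; Heard noises only store a look-at rotation, as the turning logic is disconnected.
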(event OnSeePawn(PawnSensing)
  (params (Pawn :type Pawn%20Object%20Reference))
  (if (Pawn|IsPlayerControlled Pawn)
    (AI|AIMoveTo self "0, 0, 0" Pawn 7e+01 false
      (:OnSuccess
        (bind _asbp_game_mode_main_game (Utilities|Casting|CastToBP_GameMode_MainGame (Game|GetGameMode)))
        (Default|GameEnd _asbp_game_mode_main_game false self)))))

(event OnHearNoise(PawnSensing)
  (params (Instigator :type Pawn%20Object%20Reference) (Location :type Vector%20%28by%20ref%29 :default "0, 0, 0") (Volume :type Float%20%28single-precision%29))
  (Variables|Default|SetLookAt (Math|Rotator|FindLookatRotation (Transformation|GetActorLocation) Location)))

(event EventOnDeath
  (Physics|SetSimulatePhysics (Variables|Character|GetMesh) true)
  (bind _asbp_game_mode_main_game (Utilities|Casting|CastToBP_GameMode_MainGame (Game|GetGameMode)))
  (Default|NPCKilled _asbp_game_mode_main_game)
  (Utilities|FlowControl|Delay 3.0)
  (Actor|DestroyActor))

(event EventTick
  (params (DeltaSeconds :type Float%20%28single-precision%29)))

(event EventBeginPlay
  (Rendering|Components|TextRender|SetText (Variables|Default|GetTextRender) (Utilities|Text|ToText(String) (Utilities|GetObjectName self))))

(fn ConstructionScript)