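; Main game mode that tallies enemies, collectables and power-ups, counting actors with the matching interfaces at BeginPlay.
; Events increment the current counts for kills, collections and power-up uses.
; A kill triggers a win when the enemy count equals the power-up total, not the enemy total.
; GameEnd only prints a win message, or a loss message naming the instigator.
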(event Custom|PowerUpUsed
  (Math|Integer|IncrementInt (Variables|Default|GetCurrentPowerupCount)))

(event Custom|GameEnd
  (params (DidPlayerWin :type Boolean) (Instigator :type Actor%20Object%20Reference))
  (Development|PrintString (select DidPlayerWin "You Won!" (Utilities|String|Append "You've Lost To " (Utilities|GetObjectName Instigator))) true true "(R=0.000000,G=1.000000,B=0.000000,A=1.000000)" 1e+01))

(event Custom|NPCKilled
  (Math|Integer|IncrementInt (Variables|Default|GetCurrentEnemyCount)
    (:%20%20
      (if (== (Variables|Default|GetCurrentEnemyCount) (Variables|Default|GetTotalPowerupCount))
        (CallFunction|GameEnd true)))))

(event Custom|CollectablesCollected
  (Math|Integer|IncrementInt (Variables|Default|GetCurrentCollectableCount)))

(event EventBeginPlay
  (bind _outactors (Actor|GetAllActorswithInterface "/Game/_Project/Pawns/BPI_Enemy.BPI_Enemy_C"))
  (Variables|Default|SetTotalEnemyCount (Utilities|Array|Length _outactors))
  (bind _outactors_2 (Actor|GetAllActorswithInterface "/Game/_Project/Items/BPI_Collectable.BPI_Collectable_C"))
  (Variables|Default|SetTotalCollectableCount (Utilities|Array|Length _outactors_2))
  (bind _outactors_3 (Actor|GetAllActorswithInterface "/Game/_Project/Items/BPI_Power.BPI_Power_C"))
  (Variables|Default|SetTotalPowerupCount (Utilities|Array|Length _outactors_3)))

(fn ConstructionScript)