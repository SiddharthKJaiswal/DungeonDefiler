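; Player HUD Blueprint that manages the game start and end screens and relays player data to the HUD widget.
; On BeginPlay it shows WBP_GameBegin with UI-only input and a visible cursor.
; UpdatePlayerData forwards values to ReferenceHUD, which is not assigned in these graphs.
; Death and win events open WBP_GameEnd in the same input mode, passing a boolean for the outcome.
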(event EventBeginPlay
  (bind _returnvalue (UserInterface|CreateWidget "/Game/_Project/UserInterface/WBP_GameBegin.WBP_GameBegin_C" (Game|Player|GetOwningPlayerController)))
  (UserInterface|Viewport|AddtoViewport _returnvalue 0)
  (Input|SetInputModeUIOnly (Game|Player|GetOwningPlayerController) _returnvalue "DoNotLock" false)
  (Variables|/Script/Engine.PlayerController|SetbShowMouseCursor (Game|Player|GetOwningPlayerController) true))

(event EventUpdatePlayerData
  (params (ValueToUpdate :type Integer) (NewValue :type Float%20%28single-precision%29))
  (Default|UpdatePlayerData (Variables|Default|GetReference_HUD) NewValue ValueToUpdate))

(event EventUpdatePlayerDeath
  (bind _returnvalue (UserInterface|CreateWidget "/Game/_Project/UserInterface/WBP_GameEnd.WBP_GameEnd_C" (Game|Player|GetOwningPlayerController)))
  (Default|SetGameState _returnvalue false)
  (UserInterface|Viewport|AddtoViewport _returnvalue 0)
  (Input|SetInputModeUIOnly (Game|Player|GetOwningPlayerController) _returnvalue "DoNotLock" false)
  (Variables|/Script/Engine.PlayerController|SetbShowMouseCursor (Game|Player|GetOwningPlayerController) true))

(event EventUpdatePlayerWin
  (bind _returnvalue (UserInterface|CreateWidget "/Game/_Project/UserInterface/WBP_GameEnd.WBP_GameEnd_C" (Game|Player|GetOwningPlayerController)))
  (Default|SetGameState _returnvalue true)
  (UserInterface|Viewport|AddtoViewport _returnvalue 0)
  (Input|SetInputModeUIOnly (Game|Player|GetOwningPlayerController) _returnvalue "DoNotLock" false)
  (Variables|/Script/Engine.PlayerController|SetbShowMouseCursor (Game|Player|GetOwningPlayerController) true))

(fn ConstructionScript)